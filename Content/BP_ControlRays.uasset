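; BP_ControlRays is the controller actor for a 3D Bellhop underwater acoustics visualization, showing sound rays, ocean geometry and a transmission loss UI.
; It spawns ray actors with Niagara tracers and attached noise, builds procedural bottom and surface meshes, and feeds depth range to a colorbar.
; Moving the source along its spline-drawn path, by grab point or by depth, updates Bellhop and rebuilds rays.
; EndPlay restores the original source position.
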(event `self.ReceiveEndPlay`
  (params (EndPlayReason :type "EEndPlayReason Enum" :default "Destroyed"))
  (`self.MoveSource3D` (`.Bellhop` (`self.Bellhop`)) (`self.source_id`) (`self.OriginalPosition`)))

(event `self.ReceiveBeginPlay`
  (`|ExecutionSequence`
    (:`then_0`
      ;[1 1 1] Get first - Main bellhop acoustic library interface
      (bind _returnvalue (`GameplayStatics.GetActorOfClass` null))
      (set `self.Bellhop` null _returnvalue))
    (:`then_1`
      ;[1 1 1] UI Widgets
      (bind _returnvalue_2 (`|CreateWidget` "/Game/UI/UI_TransmissionLoss3D.UI_TransmissionLoss3D_C" (`GameplayStatics.GetPlayerController` 0)))
      (bind _output_get (set `self.MainUI` _returnvalue_2))
      (`UserWidget.AddToViewport` _output_get 0))
    (:`then_2`
      ;[1 1 1] Depth Colorbar initialization
      (bind _returnvalue_3 (`GameplayStatics.GetActorOfClass` "/Game/UI/BP_ColorBarTarget.BP_ColorBarTarget_C"))
      (set `self.ColorBarView` _returnvalue_3))))

(event `MoveSource`
  (bind _sourcelocations (`self.SourceLocations`))
  ;[1 1 1] Move the source along the planned path
  (bind _result (`/Engine/EditorBlueprintResources/StandardMacros.IncrementInt` (`self.SourceLocationStep`))
    (:`  `
      (bind _output (`|GetArrayItem` _sourcelocations (mod _result (`KismetArrayLibrary.Array_Length` _sourcelocations))))
      (`self.MoveSource3D` (`.Bellhop` (`self.Bellhop`)) (`self.source_id`) _output)
      (bind _outactors (`GameplayStatics.GetAllActorsOfClass` null))
      (for (_array_element _array_index) _outactors
        (`self.CreateStructure` _array_element _array_index (`self.M_RayTrace`) (`self.Structure Radius`)))
      (`self.SetSoundSourceMarker` _output))))

(event `FlattenSSP`
  ;[1 1 1] Mostly testing - Flatten the SSP
  (`self.TestingFlattenSoundSpeedProfile` (`.Bellhop` (`self.Bellhop`)))
  (bind _outactors (`GameplayStatics.GetAllActorsOfClass` null))
  (for (_array_element _array_index) _outactors
    (`self.CreateStructure` _array_element _array_index (`self.M_RayTrace`) (`self.Structure Radius`))))

(event `SpawnRay`
  (bind _ssourcepath (`self.SSourcePath`))
  (`|ExecutionSequence`
    (:`then_0`
      (`self.ShowRays`))
    (:`then_1`
      (`self.ShowOcean`))
    (:`then_2`
      ;[1 1 1] Source path
      (`SplineComponent.ClearSplinePoints` (`self.SSourcePath`) true)
      (for _array_element (`self.SourceLocations`)
        (`SplineComponent.AddSplinePoint` (`self.SSourcePath`) (`KismetMathLibrary.MakeVector` (.x _array_element) (.y _array_element) (* (.z _array_element) -1.0)) "World" true))
      (for _index (range (+ (- (`SplineComponent.GetNumberOfSplinePoints` (`self.SSourcePath`)) 2) 1))
        (bind _returnvalue (`AddComponent|NODE_AddSplineMeshComponent-0` :`bManualAttachment` true))
        (`SplineMeshComponent.SetForwardAxis` _returnvalue "Y" true)
        (bind (_location _tangent) (`SplineComponent.GetLocationAndTangentAtSplinePoint` _ssourcepath _index "World"))
        (bind (_location_2 _tangent_2) (`SplineComponent.GetLocationAndTangentAtSplinePoint` _ssourcepath (+ _index 1) "World"))
        (`SplineMeshComponent.SetStartAndEnd` _returnvalue _location _tangent _location_2 _tangent_2 true)
        (`PrimitiveComponent.SetMaterial` _returnvalue 0 "/Game/Assets/M_SourcePath.M_SourcePath")))))

(event `self.ReceiveActorBeginCursorOver`
  ;[0.1667 0.1667 0.1667] Check if the cursor hovering over the Grab Object
  (set `self.CursorIsHovering` true)
  (`KismetSystemLibrary.PrintString` "Hovering over grab point" false))

(event `self.ReceiveActorEndCursorOver`
  ;[0.1667 0.1667 0.1667] Check if the cursor hovering over the Grab Object
  (set `self.CursorIsHovering` false)
  (`KismetSystemLibrary.PrintString` "Cursor exiting" false))

(event `TurnOffSurface`
  (`SceneComponent.SetVisibility` (`self.FlatSurface`) false false)
  (`SceneComponent.SetVisibility` (`self.Surface`) false false))

(fn `ChangeSoundSourceDepth`
  (params (NewDepth :type "Float (double-precision)"))
  (bind (_bellhop _bellhop_2) (`self.Bellhop`))
  (`self.MoveSource3D` _bellhop_2 (`self.source_id`) (`KismetMathLibrary.MakeVector` (.x (`self.CurrentSoundSourcePosition`)) (.y (`self.CurrentSoundSourcePosition`)) NewDepth))
  (`self.ReconstructRays`)
  (bind _returnvalue (`self.GetSourceLocation` _bellhop_2 (`self.source_id`)))
  (set `self.CurrentSoundSourcePosition` _returnvalue))

(fn `ClearOcean`
  (bind _outactors (`GameplayStatics.GetAllActorsOfClass` null))
  (for _array_element _outactors
    (`self.K2_DestroyActor` _array_element))
  (`ProceduralMeshComponent.ClearAllMeshSections` (`self.Bottom`))
  (`ProceduralMeshComponent.ClearAllMeshSections` (`self.Surface`)))

(fn `ClearRays`
  (bind _outactors (`GameplayStatics.GetAllActorsOfClass` null))
  (for _array_element _outactors
    (`self.K2_DestroyActor` _array_element))
  (set `self.RayMode` false))

(fn `FindLongestRay`
  (returns (NPoints :type Integer) (RayID :type Integer))
  (locals (MaxNPoints :type Integer) (LongestRayID :type Integer))
  (bind _maxnpoints (`local.MaxNPoints`))
  (bind _outactors (`GameplayStatics.GetAllActorsOfClass` null))
  (for (_ _array_index) _outactors
    (if (> (`self.GetNPoints` (`.Bellhop` (`self.Bellhop`)) _array_index) _maxnpoints)
      (set `local.MaxNPoints` 0)
      (bind _output_get (set `local.LongestRayID` _array_index))))
  (return _maxnpoints _output_get))

(fn `Finished Moving Grab Point`
  (bind _result (`/Engine/EditorBlueprintResources/StandardMacros.NegateFloat` (.z (`SceneComponent.K2_GetComponentLocation` (`/Game/Assets/BP_SoundMover.DefaultSceneRoot` (`self.SoundSourceMover`)))))
    (:`  `
      (bind _returnvalue (`KismetMathLibrary.MakeVector` (.x (`SceneComponent.K2_GetComponentLocation` (`/Game/Assets/BP_SoundMover.DefaultSceneRoot` (`self.SoundSourceMover`)))) (.y (`SceneComponent.K2_GetComponentLocation` (`/Game/Assets/BP_SoundMover.DefaultSceneRoot` (`self.SoundSourceMover`)))) _result))
      (`self.MoveSource3D` (`.Bellhop` (`self.Bellhop`)) (`self.source_id`) _returnvalue)
      (bind _outactors (`GameplayStatics.GetAllActorsOfClass` null))
      (for (_array_element _array_index) _outactors
        (`self.CreateStructure` _array_element _array_index (`self.M_RayTrace`) (`self.Structure Radius`)))
      (`self.SetSoundSourceMarker` _returnvalue)
      (set `self.CurrentSoundSourcePosition` _returnvalue)
      (`self.GetSourceLocation` (`.Bellhop` (`self.Bellhop`)) (`self.source_id`)))))

(fn `GetMaxArrivalTime`
  (returns (MaxArrivalTime :type "Float (double-precision)"))
  (bind _returnvalue (`self.GetMaxArrivalTime` (`.Bellhop` (`self.Bellhop`))))
  (`KismetSystemLibrary.PrintString` (`KismetStringLibrary.Conv_DoubleToString` _returnvalue))
  (return _returnvalue))

(fn `ReconstructRays`
  (bind _outactors (`GameplayStatics.GetAllActorsOfClass` null))
  (for (_array_element _array_index) _outactors
    (`self.CreateStructure` _array_element _array_index (`self.M_RayTrace`) (`self.Structure Radius`))))

(fn `SetSoundSourceMarker`
  (params (Location :type "Vector Structure"))
  (bind _returnvalue (`KismetMathLibrary.Conv_VectorToTransform` Location))
  (bind _outactors (`GameplayStatics.GetAllActorsOfClass` "/Game/BP_SoundSourceMarker.BP_SoundSourceMarker_C"))
  (if (<= (`KismetArrayLibrary.Array_Length` _outactors) 0)
    (bind _returnvalue_2 (`|SpawnActorFromClass` "/Game/BP_SoundSourceMarker.BP_SoundSourceMarker_C" _returnvalue "Undefined" "MultiplyWithRoot" null null))
    (bind _output_get (set `self.SoundSourceMarker` _returnvalue_2))
    (`self.SetOwner` _output_get (`GameplayStatics.GetPlayerPawn` 0))
    (else
      (`self.K2_SetActorTransform` (`self.SoundSourceMarker`) _returnvalue false false))))

(fn `ShowOcean`
  (bind _flatsurface (`self.FlatSurface`))
  (`self.ClearOcean`)
  (bind _returnvalue (`|SpawnActorFromClass` null (`self.GetTransform`) "Undefined" "OverrideRootScale" null null))
  (bind (_output_get _output_get_2) (set `self.BottomActor` null _returnvalue))
  (`self.ReadFile` _output_get_2 (`self.BellhopRootName`) (`self.Ocean3D`) (`self.Ray3D`))
  (bind _returnvalue_2 (`self.GetNPointsX` _returnvalue))
  (bind _returnvalue_3 (`self.GetNPointsY` _returnvalue))
  (bind _returnvalue_4 (`self.GetBottomMeshVertices` _returnvalue))
  (bind _returnvalue_5 (`self.GetHeightMapUV` _returnvalue))
  (bind _triangles (`KismetProceduralMeshLibrary.CreateGridMeshWelded` _returnvalue_2 _returnvalue_3))
  (`ProceduralMeshComponent.CreateMeshSection_LinearColor` :`self` (`self.Bottom`) :`Vertices` _returnvalue_4 :`Triangles` _triangles :`UV0` _returnvalue_5)
  (`PrimitiveComponent.SetMaterial` (`self.Bottom`) 0 (`self.M_Bottom`))
  (`/Game/UI/BP_ColorBarTarget.UpdateColorBar` (`self.ColorBarView`) (`self.GetZMin` (`.BottomActor` (`self.BottomActor`))) (`self.GetZMax` (`.BottomActor` (`self.BottomActor`))))
  (bind (_triangles_2 _vertices _uvs) (`KismetProceduralMeshLibrary.CreateGridMeshWelded` 2 2 1.0))
  (for _index (range 4)
    (bind _output (`|GetArrayItem` _returnvalue_4))
    (bind (_returnvalue_x _returnvalue_y) (`KismetMathLibrary.BreakVector` (+ _output (* (+ (`|GetArrayItem` _vertices _index) (0.5 0.5 0.0)) (- (`|GetArrayItem` _returnvalue_4 (- (`KismetArrayLibrary.Array_Length` _returnvalue_4) 1)) _output)))))
    (`KismetArrayLibrary.Array_Set` _vertices _index (`KismetMathLibrary.MakeVector` _returnvalue_x _returnvalue_y)))
  (`ProceduralMeshComponent.CreateMeshSection_LinearColor` :`self` (`self.Surface`) :`Vertices` _vertices :`Triangles` _triangles_2 :`UV0` _uvs)
  (`PrimitiveComponent.SetMaterial` (`self.Surface`) 0 (`self.M_Surface`))
  (`ProceduralMeshComponent.CreateMeshSection_LinearColor` :`self` _flatsurface :`Vertices` _vertices :`Triangles` _triangles_2 :`UV0` _uvs)
  (`PrimitiveComponent.SetMaterial` _flatsurface 0 (`self.M_FlatSurface`)))

(fn `ShowRays`
  (bind (_bellhop _bellhop_2) (`self.Bellhop`))
  (`self.ClearRays`)
  (for _index (range (+ (`self.NumberRays`) 1))
    (bind _returnvalue (`|SpawnActorFromClass` null (`self.GetTransform`) "Undefined" "MultiplyWithRoot" null null))
    (`self.ReadFile` _bellhop_2 (`self.BellhopRootName`) (`self.Ocean3D`) (`self.Ray3D`))
    (`self.CreateStructure` _returnvalue _index (`self.M_RayTrace`) (`self.Structure Radius`))
    (set `/Game/BP_ControlRays.WorldParameters` "/Game/Assets/MP_TransmissionLoss3D.MP_TransmissionLoss3D" _returnvalue)
    (set `/Game/BP_ControlRays.Particle` "/Game/Assets/NS_Tracer2.NS_Tracer2" _returnvalue)
    (`self.AttachParticles` _returnvalue)
    (bind _spherevisual (`/Game/BP_ControlRays.SphereVisual` _returnvalue))
    (`GameplayStatics.SpawnSoundAttached` "/Game/Assets/Sounds/WhiteNoise.WhiteNoise" _spherevisual "None" (0.0 0.0 0.0) (struct) "KeepRelativeOffset" false 1.0 1.0 0.0 null null)
    (`SceneComponent.SetHiddenInGame` _spherevisual true false)
    (bind _returnvalue_2 (`self.GetSourceLocation` (`.Bellhop` (`self.Bellhop`)) (`self.source_id`)))
    (`SceneComponent.K2_AddWorldOffset` (`self.Source`) _returnvalue_2 false false)
    (`KismetArrayLibrary.Array_Add` (`.AllRays` (`self.AllRays`)) _returnvalue)
    (`/Engine/EditorBlueprintResources/StandardMacros.DoOnce` false
      (:`Completed`
        (bind _result (`/Engine/EditorBlueprintResources/StandardMacros.DecrementInt` (`self.GetNRays` _bellhop_2))
          (:`  `
            (set `self.NumberRays` _result)
            (bind _returnvalue_3 (`self.GetSourceLocation` _bellhop_2 (`self.source_id`)))
            (set `self.OriginalPosition` _returnvalue_3)
            (set `self.CurrentSoundSourcePosition` _returnvalue_3))))))
  (`self.UpdateRayTakeoffs`)
  (`self.SetSoundSourceMarker` _returnvalue_2)
  (set `self.RayMode` true)
  (`KismetMaterialLibrary.SetScalarParameterValue` null "None" 1.0))

(fn `StartArrowAxisDrag`
  (params (Component :type "ActorComponent Object Reference"))
  (locals (`Source Depth` :type "Vector Structure" :default (0.0 0.0 0.0)))
  (bind _returnvalue (`KismetSystemLibrary.GetDisplayName` Component))
  (bind _returnvalue_2 (`self.GetSourceLocation` (`.Bellhop` (`self.Bellhop`)) (`self.source_id`)))
  (set `local.Source Depth` _returnvalue_2)
  (`KismetSystemLibrary.PrintString` _returnvalue)
  (switch `string` _returnvalue))

(fn `TurnOffNiagaraParticles`
  (for _array_element (`self.AllParticles`)
    (`ActorComponent.Deactivate` _array_element)))

(fn `TurnOnAllParticles`
  (for _array_element (`self.AllParticles`)
    (`ActorComponent.Activate` _array_element true)))

(fn `UpdateRayTakeoffs`
  (bind (_low _high _n) (`self.GetRayAltitudes` (`.Bellhop` (`self.Bellhop`))))
  (bind (_low_2 _high_2 _n_2) (`self.GetRayAzimuths` (`.Bellhop` (`self.Bellhop`))))
  (`|ExecutionSequence`
    (:`then_0`
      ;[1 1 1] Altitudes
      (`|ExecutionSequence`
        (:`then_0`
          (set `self.AltitudeLow` _low))
        (:`then_1`
          (set `self.AltitudeHigh` _high))
        (:`then_2`
          (set `self.AltitudeCount` _n))))
    (:`then_1`
      ;[1 1 1] Azimuths
      (`|ExecutionSequence`
        (:`then_0`
          (set `self.AzimuthLow` _low_2))
        (:`then_1`
          (set `self.AzimuthHigh` _high_2))
        (:`then_2`
          (set `self.AzimuthCount` _n_2))))))

(fn `UserConstructionScript`)