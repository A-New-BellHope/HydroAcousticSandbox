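; Actor that visualizes 3D transmission loss data as procedural meshes in three views: horizontal pancakes, bearing spokes and concentric cylinders.
; Each Draw function clears its view, spawns a fresh TransmissionLoss3D actor for dimensions, vertices and textures, then builds one mesh section and dynamic material per slice.
; Spokes draw only every fourth bearing as a hack.
; Each new mesh shifts to the source's XY position; horizontal and cylinder maxima feed a material parameter collection.
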(fn `ClearCylindrical`
  (`ProceduralMeshComponent.ClearAllMeshSections` (`self.TransmissionLossCylindrical`)))

(fn `ClearHorizontal`
  (`ProceduralMeshComponent.ClearAllMeshSections` (`self.TransmissionLossHorizontal`)))

(fn `ClearSpoke`
  (`ProceduralMeshComponent.ClearAllMeshSections` (`self.TransmissionLossSpoke`)))

(fn `DrawCylindrical`
  (locals (NewLocalVar :type Integer :default 0))
  (bind _radials (`self.Radials`))
  (`self.ClearCylindrical`)
  (`self.UpdateTransmissionLoss`)
  (bind _returnvalue (`AddComponent|NODE_AddProceduralMeshComponent-3`))
  (set `self.TransmissionLossCylindrical` _returnvalue)
  ;[1 1 1] Construct the Cylinders projected in space
  (for _index (range _radials)
    (set `self.radial` _index)
    (bind (_triangles _vertices _uvs) (`KismetProceduralMeshLibrary.CreateGridMeshWelded` 2 (`self.Bearings`)))
    (bind _returnvalue_2 (`TransmissionLoss3D.GetCylinder` (`self.TLoss`) (`self.radial`)))
    (`ProceduralMeshComponent.CreateMeshSection_LinearColor` :`self` (`self.TransmissionLossCylindrical`) :`SectionIndex` (`self.radial`) :`Vertices` _returnvalue_2 :`Triangles` _triangles :`UV0` _uvs)
    (bind _returnvalue_3 (`PrimitiveComponent.CreateDynamicMaterialInstance` (`self.TransmissionLossCylindrical`) (`self.radial`) "/Game/TransmissionLoss/M_TransmissionLoss3D.M_TransmissionLoss3D" "None"))
    (`TransmissionLoss3D.UpdateTextureCylinder` (`self.TLoss`) _returnvalue_3 (`self.radial`))
    (`MaterialInstanceDynamic.SetScalarParameterValue` _returnvalue_3 "ID" (`KismetMathLibrary.Conv_IntToDouble` (`self.radial`))))
  (`KismetMaterialLibrary.SetScalarParameterValue` "/Game/Assets/MP_TransmissionLoss3D.MP_TransmissionLoss3D" "RadialMaximum" (`KismetMathLibrary.Conv_IntToDouble` (+ _radials -1)))
  (`SceneComponent.K2_AddLocalOffset` (`self.TransmissionLossCylindrical`) (* (`TransmissionLoss3D.GetSourcePosition` (`self.TLoss`) (`self.Source ID`)) (1.0 1.0 0.0)) false false))

(fn `DrawHorizontal`
  (bind _pancakes (`self.Pancakes`))
  (`self.ClearHorizontal`)
  (`self.UpdateTransmissionLoss`)
  (bind _returnvalue (`AddComponent|NODE_AddProceduralMeshComponent-5`))
  (set `self.TransmissionLossHorizontal` _returnvalue)
  ;[1 1 1] Construct the Cylinders projected in space
  (for _index (range _pancakes)
    (set `self.pancake` _index)
    (bind (_triangles _vertices _uvs) (`KismetProceduralMeshLibrary.CreateGridMeshWelded` 2 (`self.Bearings`)))
    (bind _returnvalue_2 (`TransmissionLoss3D.GetHorizontal` (`self.TLoss`) (`self.pancake`)))
    (`ProceduralMeshComponent.CreateMeshSection_LinearColor` :`self` (`self.TransmissionLossHorizontal`) :`SectionIndex` (`self.pancake`) :`Vertices` _returnvalue_2 :`Triangles` _triangles :`UV0` _uvs)
    (bind _returnvalue_3 (`PrimitiveComponent.CreateDynamicMaterialInstance` (`self.TransmissionLossHorizontal`) (`self.pancake`) "/Game/TransmissionLoss/M_TransmissionLossHorizontal.M_TransmissionLossHorizontal" "None"))
    (`TransmissionLoss3D.UpdateTextureHorizontal` (`self.TLoss`) _returnvalue_3 (`self.pancake`))
    (`MaterialInstanceDynamic.SetScalarParameterValue` _returnvalue_3 "HorizontalID" (`KismetMathLibrary.Conv_IntToDouble` (`self.pancake`))))
  (`KismetMaterialLibrary.SetScalarParameterValue` "/Game/Assets/MP_TransmissionLoss3D.MP_TransmissionLoss3D" "HorizontalMaximum" (`KismetMathLibrary.Conv_IntToDouble` (+ _pancakes -1)))
  (`SceneComponent.K2_AddLocalOffset` (`self.TransmissionLossHorizontal`) (* (`TransmissionLoss3D.GetSourcePosition` (`self.TLoss`) (`self.Source ID`)) (1.0 1.0 0.0)) false false))

(fn `DrawSpoke`
  (`self.ClearSpoke`)
  (`self.UpdateTransmissionLoss`)
  (bind _returnvalue (`AddComponent|NODE_AddProceduralMeshComponent-2`))
  (set `self.TransmissionLossSpoke` _returnvalue)
  (for _index (range (`self.Bearings`))
    (bind _output_get (set `self.bearing` _index))
    (if (== (mod _output_get 4) 0)
      (bind (_triangles _vertices _uvs) (`KismetProceduralMeshLibrary.CreateGridMeshSplit` 2 2 100.0))
      (bind _returnvalue_2 (`TransmissionLoss3D.GetCorners` (`self.TLoss`) (`self.bearing`)))
      (`ProceduralMeshComponent.CreateMeshSection_LinearColor` :`self` (`self.TransmissionLossSpoke`) :`SectionIndex` (`self.bearing`) :`Vertices` _returnvalue_2 :`Triangles` _triangles :`UV0` _uvs)
      (bind _returnvalue_3 (`PrimitiveComponent.CreateDynamicMaterialInstance` (`self.TransmissionLossSpoke`) (`self.bearing`) "/Game/TransmissionLoss/M_TransmissionLoss3D.M_TransmissionLoss3D" "None"))
      (`TransmissionLoss3D.UpdateTextureBearing` (`self.TLoss`) _returnvalue_3 (`self.bearing`))))
  (`SceneComponent.K2_AddLocalOffset` (`self.TransmissionLossSpoke`) (* (`TransmissionLoss3D.GetSourcePosition` (`self.TLoss`) (`self.Source ID`)) (1.0 1.0 0.0)) false false))

(fn `UpdateTransmissionLoss`
  (bind _returnvalue (`GameplayStatics.GetActorOfClass` "BP_SpawnTransmissionLoss3D_C"))
  (bind _returnvalue_2 (`|SpawnActorFromClass` "/Script/bellhop.TransmissionLoss3D" (`self.GetTransform` _returnvalue) "Undefined" "MultiplyWithRoot" null null))
  (bind _output_get (set `self.TLoss` _returnvalue_2))
  (`|ExecutionSequence`
    (:`then_0`
      (`TransmissionLoss3D.UpdateTransmissionLoss` _output_get))
    (:`then_1`
      (bind _returnvalue_3 (`TransmissionLoss3D.GetNumBearings` _output_get))
      (set `self.Bearings` _returnvalue_3))
    (:`then_2`
      (bind _returnvalue_4 (`TransmissionLoss3D.GetWidth` _output_get))
      (set `self.Pancakes` _returnvalue_4))
    (:`then_3`
      (bind _returnvalue_5 (`TransmissionLoss3D.GetHeight` _output_get))
      (set `self.Radials` _returnvalue_5))))

(fn `UserConstructionScript`)