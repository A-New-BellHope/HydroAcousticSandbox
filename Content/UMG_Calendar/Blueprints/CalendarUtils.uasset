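; Blueprint function library of helpers for a UMG calendar widget.
; It validates dates and year ranges, tests whether a date falls within a range, and steps to the first day of the next or previous month.
; Weekdays come from Zeller's congruence, shifted from its Saturday-first index to a Sunday- or Monday-first week.
; A separate helper applies a style struct's font, color, shadow and strike brush to a text block.
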(fn `GetDayOfWeek`
  (params (CurrentDay :type "DateTime Structure") (WeekStartsOnMonday :type Boolean))
  (returns (DayOfWeekIndex :type Integer))
  (bind _dayint (`self.ZellerCongruence` CurrentDay (`local.__WorldContext`)))
  (bind _returnvalue (select `bool` (== _dayint 0) :`false` (- _dayint 1) :`true` 6))
  (return (select `bool` WeekStartsOnMonday :`false` _returnvalue :`true` (select `bool` (== _returnvalue 0) :`false` (- _returnvalue 1) :`true` 6))))

(fn `GetNextMonth`
  (params (CurrentMonth :type "DateTime Structure"))
  (returns (NextMonth :type "DateTime Structure"))
  (locals (NextMonthIndex :type Integer) (NextMonthYear :type Integer))
  (bind _returnvalue (`KismetMathLibrary.GetMonth` CurrentMonth))
  (bind _returnvalue_2 (`KismetMathLibrary.GetYear` CurrentMonth))
  (if (== _returnvalue 12)
    (set `local.NextMonthIndex` 1)
    (set `local.NextMonthYear` (+ _returnvalue_2 1))
    (else
      (set `local.NextMonthIndex` (+ _returnvalue 1))
      (set `local.NextMonthYear` _returnvalue_2)))
  (return (`KismetMathLibrary.MakeDateTime` (`local.NextMonthYear`) (`local.NextMonthIndex`) 1)))

(fn `GetPreviousMonth`
  (params (CurrentMonth :type "DateTime Structure"))
  (returns (PreviousMonth :type "DateTime Structure"))
  (locals (PreviousMonthIndex :type Integer) (PreviousMonthYear :type Integer))
  (bind _returnvalue (`KismetMathLibrary.GetMonth` CurrentMonth))
  (bind _returnvalue_2 (`KismetMathLibrary.GetYear` CurrentMonth))
  (if (== _returnvalue 1)
    (set `local.PreviousMonthIndex` 12)
    (set `local.PreviousMonthYear` (- _returnvalue_2 1))
    (else
      (set `local.PreviousMonthIndex` (- _returnvalue 1))
      (set `local.PreviousMonthYear` _returnvalue_2)))
  (return (`KismetMathLibrary.MakeDateTime` (`local.PreviousMonthYear`) (`local.PreviousMonthIndex`) 1)))

(fn `IsCalendarDateRangeValid`
  (params (Input :type "/Game/UMG_Calendar/Blueprints/CalendarDateRange Structure"))
  (returns (IsValid :type Boolean))
  (bind ___worldcontext (`local.__WorldContext`))
  ;[1 1 1] Range is valid if both inpput year are valid and if max year is greater or equal to min year
  (return (and (>= Input_MaxYear_8_EB5657DF424B10D50D26BDA5BB409764 Input_MinYear_4_5280C3764CBDFB930D7A9A97E37DDE52) (and (`self.IsCalendarDateValid` 1 Input_MinYear_4_5280C3764CBDFB930D7A9A97E37DDE52 ___worldcontext) (`self.IsCalendarDateValid` 1 Input_MaxYear_8_EB5657DF424B10D50D26BDA5BB409764 ___worldcontext)))))

(fn `IsCalendarDateValid`
  (params (Month :type Integer) (Year :type Integer))
  (returns (IsValid :type Boolean))
  (return (and (`KismetMathLibrary.InRange_IntInt` Month 1 12) (> Year 1))))

(fn `IsDateWithinCalendarRange`
  (params (DateToTest :type "DateTime Structure") (RangeToTest :type "/Game/UMG_Calendar/Blueprints/CalendarDateRange Structure"))
  (returns (Within :type Boolean))
  (bind (_minyear _maxyear) (break `/Game/UMG_Calendar/Blueprints/CalendarDateRange` RangeToTest))
  (return (and (>= DateToTest (`KismetMathLibrary.MakeDateTime` _minyear 1 1)) (< DateToTest (`self.GetNextMonth` (`KismetMathLibrary.MakeDateTime` _maxyear 12 31) (`local.__WorldContext`))))))

(fn `SetTextBlockStyle`
  (params (TB :type "TextBlock Object Reference") (TBStyle :type "TextBlockStyle Structure"))
  (bind (_font _colorandopacity _shadowoffset _shadowcolorandopacity _highlightcolor _highlightshape _strikebrush) (break `TextBlockStyle` TBStyle))
  (`TextBlock.SetFont` TB _font)
  (`TextBlock.SetColorAndOpacity` TB _colorandopacity)
  (`TextBlock.SetShadowOffset` TB _shadowoffset)
  (`TextBlock.SetShadowColorAndOpacity` TB _shadowcolorandopacity)
  (`TextBlock.SetStrikeBrush` TB _strikebrush))

(fn `ZellerCongruence`
  (params (CurrentTime :type "DateTime Structure"))
  (returns (DayInt :type Integer))
  (locals (ShiftedMonth :type Integer) (ShiftedYear :type Integer) (Day :type Integer) (Month :type Integer) (Decade :type Integer) (Century :type Integer))
  (bind _returnvalue (`KismetMathLibrary.GetMonth` CurrentTime))
  (bind _returnvalue_2 (`KismetMathLibrary.GetYear` CurrentTime))
  (bind _shiftedyear (`local.ShiftedYear`))
  ;[1 1 1] Calculate the day of the week for any date using Zeller's congruence formula. See https://en.wikipedia.org/wiki/Zeller%27s_congruence / Beware, this function returns week day index with saturday being the first day ie if week day is saturday, returns 0
  (if (<= _returnvalue 2)
    (set `local.ShiftedMonth` (+ _returnvalue 12))
    (set `local.ShiftedYear` (- _returnvalue_2 1))
    (else
      (set `local.ShiftedMonth` _returnvalue)
      (set `local.ShiftedYear` _returnvalue_2)))
  (set `local.Day` (`KismetMathLibrary.GetDay` CurrentTime))
  (set `local.Month` (`local.ShiftedMonth`))
  (set `local.Decade` (mod _shiftedyear 100))
  (set `local.Century` (/ _shiftedyear 100))
  (return (mod (+ (`local.Day`) (/ (* (+ (`local.ShiftedMonth`) 1) 13) 5) (`local.Decade`) (/ (`local.Decade`) 4) (/ (`local.Century`) 4) (* (`local.Century`) 5)) 7)))