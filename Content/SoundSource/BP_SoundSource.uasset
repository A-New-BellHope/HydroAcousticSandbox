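; Sound source actor that drives Bellhop acoustic simulations and displays their results as rays or transmission loss.
; It moves in front of the player or to a given depth, dividing Z by the shader's ScaleZ before updating Bellhop.
; Transmission loss runs in the background behind a blocking progress widget polled on Tick.
; Bellhop's done event spawns FollowRays actors or refreshes the transmission loss display, depending on mode.
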(event `self.ReceiveBeginPlay`
  ;[1 1 1] TODO: may not need.
  (`self.EnableInput` (`GameplayStatics.GetPlayerController` 0))
  ;[1 1 1] Convenience variables
  (bind _returnvalue (`GameplayStatics.GetActorOfClass` "/Game/Assets/Sandbox/BP_Globals.BP_Globals_C"))
  (bind _output_get (set `self.Globals` _returnvalue))
  (bind _output_get_2 (set `self.Bellhop` (`/Game/Assets/Sandbox/BP_Globals.BellhopRef` _output_get)))
  (bind _returnvalue_2 (`|CreateWidget` "/Game/SoundSource/WB_BlockerTL.WB_BlockerTL_C" (`GameplayStatics.GetPlayerController` 0)))
  (bind _output_get_3 (set `self.Blocker` _returnvalue_2))
  (`UserWidget.AddToViewport` _output_get_3 9999)
  (`/Game/SoundSource/WB_BlockerTL.ShowScene` (`self.Blocker`))
  ;[1 1 1] Respond to the calculation finishing
  (add `BellhopController.OnBellhopDoneEvent` _output_get_2 (delegate `OnBellhopDone`)))

(event `OnBellhopDone`
  ;[1 1 1] Respond to the calculation finishing
  (set `self.BUpdateBlocker` false)
  (if (`BellhopController.IsRayMode` (`self.Bellhop`))
    (`self.DrawRays`)
    (elif (`BellhopController.IsTransmissionLossMode` (`self.Bellhop`))
      (`self.DrawTransmissionLoss`)
      (else
        (`KismetSystemLibrary.PrintString` "Error: only TL and ray mode are aupported."))))
  (`/Game/SoundSource/WB_BlockerTL.ShowScene` (`self.Blocker`)))

(event `self.ReceiveTick`
  (params (DeltaSeconds :type "Float (single-precision)"))
  ;[1 1 1] Update bar
  (if (`self.BUpdateBlocker`)
    (bind _returnvalue (`BellhopController.GetPercentDone` (`self.Bellhop`)))
    (`/Game/SoundSource/WB_BlockerTL.SetPercentDone` (`self.Blocker`) (`KismetMathLibrary.Conv_IntToDouble` _returnvalue))))

(fn `AdjustSoundSourceDepth`
  (params (NewDepth :type "Float (double-precision)"))
  (bind _returnvalue (`KismetMaterialLibrary.GetScalarParameterValue` "/Game/Assets/MP_TransmissionLoss3D.MP_TransmissionLoss3D" "ScaleZ")) ; compensate for shader scaling
  (bind _output_get (set `self.NewSourceLocation` (/ (`KismetMathLibrary.MakeVector` (.x (`SceneComponent.K2_GetComponentLocation` (`self.DefaultSceneRoot`))) (.y (`SceneComponent.K2_GetComponentLocation` (`self.DefaultSceneRoot`))) NewDepth) (`KismetMathLibrary.MakeVector` 1.0 1.0 _returnvalue))))
  (`SceneComponent.K2_SetWorldLocation` (`self.DefaultSceneRoot`) _output_get false false)
  (`BellhopController.MoveSource3D` (`self.Bellhop`) (`self.SourceID`) (`self.NewSourceLocation`)))

(fn `CalculateRays`
  (`|ExecutionSequence`
    (:`then_0`
      ;[1 1 1] Initialize and clean up
      (`self.ClearRays`)
      (`BellhopController.SetRayMode` (`self.Bellhop`)))
    (:`then_1`
      ;[1 1 1] Placeholder for checking parameters
      (`KismetSystemLibrary.PrintString` "TODO: add a function to check that the ray parameters are set." true true (struct :`R` 1.0 :`B` 0.403251 :`A` 1.0) 30.0))
    (:`then_2`
      ;[1 1 1] Start the bellhop background thread
      (`BellhopController.RunBellhop` (`self.Bellhop`)))))

(fn `CalculateTransmissionLoss`
  (params (TransmissionLossMode :type "ETransmissionLossMode Enum" :default "Incoherent"))
  (`|ExecutionSequence`
    (:`then_0`
      ;[1 1 1] Initialize and clean up
      (`self.ClearTransmissionLoss`)
      (`BellhopController.SetTransmissionLossMode` (`self.Bellhop`) TransmissionLossMode))
    (:`then_1`
      ;[1 1 1] Block the UI
      (`/Game/SoundSource/WB_BlockerTL.BlockScene` (`self.Blocker`))
      (`/Game/SoundSource/WB_BlockerTL.SetPercentDone` (`self.Blocker`) 0.0))
    (:`then_2`
      ;[1 1 1] Start the bellhop background thread
      (`BellhopController.BackgroundRunBellhop` (`self.Bellhop`))
      (set `self.BUpdateBlocker` true))))

(fn `ClearRays`
  (bind _outactors (`GameplayStatics.GetAllActorsOfClass` "/Script/bellhop.FollowRays"))
  (for _array_element _outactors
    (`self.K2_DestroyActor` _array_element)))

(fn `ClearTransmissionLoss`)

(fn `DrawRays`
  (for _index (range (`BellhopController.GetNRays` (`self.Bellhop`)))
    (bind _returnvalue (`|SpawnActorFromClass` "/Script/bellhop.FollowRays" (`self.GetTransform`) "Undefined" "MultiplyWithRoot" null null))
    (`FollowRays.CreateStructure` _returnvalue _index "/Game/SoundSource/M_Ray.M_Ray" (`self.Structure Radius`))
    (set `FollowRays.WorldParameters` "/Game/Assets/MP_TransmissionLoss3D.MP_TransmissionLoss3D" _returnvalue))
  (`KismetSystemLibrary.PrintString` "Done spawning rays" true true (struct :`R` 1.0 :`B` 0.685434 :`A` 1.0) 30.0))

(fn `DrawTransmissionLoss`
  (`KismetSystemLibrary.PrintString` "Completed the TL calculation" true true (struct :`R` 1.0 :`B` 0.496511 :`A` 1.0) 20.0)
  (`/Game/TransmissionLoss/BP_SpawnTransmissionLoss3D.UpdateTransmissionLoss` (`/Game/Assets/Sandbox/BP_Globals.SpawnTransmissionLossRef` (`self.Globals`))))

(fn `MoveSoundSource`
  (bind _returnvalue (`GameplayStatics.GetPlayerPawn` 0))
  (bind _returnvalue_2 (`KismetMaterialLibrary.GetScalarParameterValue` "/Game/Assets/MP_TransmissionLoss3D.MP_TransmissionLoss3D" "ScaleZ")) ; compensate for shader scaling
  (bind _output_get (set `self.NewSourceLocation` (/ (+ (`self.K2_GetActorLocation` _returnvalue) (* (`self.GetActorForwardVector` _returnvalue) (`self.SourceDistance`))) (`KismetMathLibrary.MakeVector` 1.0 1.0 _returnvalue_2))))
  (`SceneComponent.K2_SetWorldLocation` (`self.DefaultSceneRoot`) _output_get false false)
  (`BellhopController.MoveSource3D` (`self.Bellhop`) (`self.SourceID`) (`self.NewSourceLocation`)))

(fn `UserConstructionScript`)