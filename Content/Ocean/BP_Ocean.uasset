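; BP_Ocean builds the ocean environment for a Bellhop 3D acoustic simulation from real bathymetry and HYCOM sound-speed data.
; BeginPlay takes bounds from the game instance or a default, builds the seafloor procedural mesh, then requests sound speed behind a loading widget.
; When HYCOM finishes, Bellhop receives the hexahedral grid and a minimum-sound-speed depth surface is drawn, falling back to a Munk profile without data.
; DropVertical spawns textured sound-speed profile cylinders.
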(event `self.ReceiveBeginPlay`
  (bind (_bottomboundary_north _bottomboundary_east _bottomboundary_south _bottomboundary_west _bottomboundary_time) (break `/Game/Ocean/S_OceanBounds` (`self.BottomBoundary`)))
  (`|ExecutionSequence`
    (:`then_0`
      ;[1 1 1] Initialize objects or find references
      (bind _returnvalue (`|SpawnActorFromClass` "/Script/netcdfunreal.Bathymetry" (`self.Zero`) "Undefined" "MultiplyWithRoot" null null))
      (set `self.BathymetryReader` _returnvalue)
      (bind _returnvalue_2 (`|SpawnActorFromClass` "/Script/bellhop.Bottom" (`self.Zero`) "Undefined" "MultiplyWithRoot" null null))
      (set `self.Bottom` _returnvalue_2)
      (add `Bathymetry.OnHYCOMDoneEvent` (`self.BathymetryReader`) (delegate `HYCOMDone`))
      (bind _returnvalue_3 (`|CreateWidget` "/Game/Ocean/UI_LoadingSoundSpeed.UI_LoadingSoundSpeed_C" (`GameplayStatics.GetPlayerController` 0)))
      (bind _output_get (set `self.Blocker` _returnvalue_3))
      (`UserWidget.AddToViewport` _output_get 9999)
      (bind _returnvalue_4 (`|SpawnActorFromClass` "/Script/bellhop.SSPVolume" (`self.Zero`) "Undefined" "MultiplyWithRoot" null null))
      (set `self.SSPVolume` _returnvalue_4))
    (:`then_1`
      ;[1 1 1] Initialize bellhop in 3d
      ; TODO: should do this somewhere else
      (`BellhopController.SetupDefaults` (`self.Bellhop`) (`self.O3D`) (`self.R3D`)))
    (:`then_2`
      (`self.UpdateGlobalBounds`)
      ;[1 1 1] Update simulation
      (`Bathymetry.SetTiffBounds` (`self.BathymetryReader`) _bottomboundary_north _bottomboundary_east _bottomboundary_south _bottomboundary_west)
      (`self.RunBathymetry` _bottomboundary_north _bottomboundary_east _bottomboundary_south _bottomboundary_west)
      (`/Game/Ocean/UI_LoadingSoundSpeed.BlockScene` (`self.Blocker`))
      (`Bathymetry.GetEarthSoundSpeed` (`self.BathymetryReader`) (`self.Actual North`) (`self.Actual East`) (`self.Actual South`) (`self.Actual West`) _bottomboundary_time))))

(event `HYCOMDone`
  ;[1 1 1] Run after the hycom download finishes
  (`self.HandleHYCOMDone`)
  (`/Game/Ocean/UI_LoadingSoundSpeed.ShowScene` (`self.Blocker`)))

(event `TestWriteDone`
  ;[1 1 1] Testing only
  (`KismetSystemLibrary.PrintString` "Test write done" true true (struct :`R` 1.0 :`B` 0.62521 :`A` 1.0) 30.0))

(fn `CheckRange`
  (params (Value :type "Float (double-precision)"))
  (returns (ValueFix :type "Float (double-precision)"))
  (locals (res :type "Float (double-precision)"))
  (bind _output_get (set `local.res` Value))
  (`|ExecutionSequence`
    (:`then_0`
      (while (< _output_get -180.0)
        (set `local.res` (+ (`local.res`) 360.0))))
    (:`then_1`
      (while (>= _output_get 180.0)
        (set `local.res` (- (`local.res`) 360.0))))
    (:`then_2`
      (return (`local.res`)))))

(fn `ClearBathymetry`
  (`ProceduralMeshComponent.ClearAllMeshSections` (`self.BottomMesh`)))

(fn `DrawSoundSpeedMinimum`
  (locals (NewLocalVar :type Boolean) (Vertices :type "Array of Vector Structure") (NGridX :type Integer :default 0) (NGridY :type Integer :default 0) (NDepth :type Integer :default 0) (SSPTemp :type "Array of Float (double-precision)"))
  (`|ExecutionSequence`
    (:`then_0`
      ;[1 1 1] Reset and grab some local variables
      (`ProceduralMeshComponent.ClearAllMeshSections` (`self.SSPSurface`))
      (set `local.NGridX` (`KismetArrayLibrary.Array_Length` (`self.HexGridX`)))
      (set `local.NGridY` (`KismetArrayLibrary.Array_Length` (`self.HexGridY`)))
      (bind _output_get (set `local.NDepth` (`KismetArrayLibrary.Array_Length` (`self.HexDepth`))))
      (`KismetArrayLibrary.Array_Resize` (`local.SSPTemp`) _output_get))
    (:`then_1`
      ;[1 1 1] Get the depth at the minimum ssp. TODO: pretty ugly to do in a blurprint
      (for _array_element (`self.HexGridX`)
        (for _array_element_2 (`self.HexGridY`)
          (for (_array_element_3 _array_index) (`self.HexDepth`)
            (bind _soundspeed (`BellhopController.GetSingleSoundSpeed` (`self.Bellhop`) (`KismetMathLibrary.MakeVector` _array_element _array_element_2 _array_element_3)))
            (`KismetArrayLibrary.Array_Set` (`local.SSPTemp`) _array_index _soundspeed))
          (`KismetArrayLibrary.Array_Add` (`local.Vertices`) (`KismetMathLibrary.MakeVector` _array_element _array_element_2 (* (`|GetArrayItem` (`self.HexDepth`) (`KismetMathLibrary.MinOfFloatArray` (`local.SSPTemp`))) -1.0))))))
    (:`then_2`
      ;[1 1 1] Draw the mesh
      (bind (_triangles _vertices _uvs) (`KismetProceduralMeshLibrary.CreateGridMeshWelded` (`local.NGridY`) (`local.NGridX`)))
      (`ProceduralMeshComponent.CreateMeshSection_LinearColor` :`self` (`self.SSPSurface`) :`Vertices` (`local.Vertices`) :`Triangles` _triangles :`UV0` _uvs)
      (`PrimitiveComponent.SetMaterial` (`self.SSPSurface`) 0 "/Game/Assets/M_ScaleSurface.M_ScaleSurface"))))

(fn `DropVertical`
  (params (Position :type "Vector Structure"))
  (locals (VerticalProfileBottom :type "Vector Structure") (VerticalProfileTop :type "Vector Structure") (VerticalProfileSamples :type Integer :default 100))
  (bind (_verticalprofilebottom_x _verticalprofilebottom_y _verticalprofilebottom_z) (`KismetMathLibrary.BreakVector` (`local.VerticalProfileBottom`)))
  (bind (_verticalprofiletop_x _verticalprofiletop_y) (`KismetMathLibrary.BreakVector` (`local.VerticalProfileTop`)))
  (set `local.VerticalProfileTop` (* Position (1.0 1.0 0.0)))
  (`|ExecutionSequence`
    (:`then_0`
      ;[1 1 1] Find the intersection.
      (set `local.VerticalProfileBottom` (`KismetMathLibrary.MakeVector` _verticalprofiletop_x _verticalprofiletop_y (`SSPVolume.GetDepthBelow` (`self.SSPVolume`) (`local.VerticalProfileTop`)))))
    (:`then_2`
      ;[1 1 1] Spawn the tube
      (bind _returnvalue (`|SpawnActorFromClass` "/Game/Assets/3DModels/BP_ProceduralCylinder.BP_ProceduralCylinder_C" (`KismetMathLibrary.MakeTransform` (`local.VerticalProfileTop`)) "Undefined" "MultiplyWithRoot" null null))
      (`/Game/Assets/3DModels/BP_ProceduralCylinder.SetHeight` _returnvalue _verticalprofilebottom_z)
      (bind _procmesh (`/Game/Assets/3DModels/BP_ProceduralCylinder.ProcMesh` _returnvalue))
      (bind _returnvalue_2 (`PrimitiveComponent.CreateDynamicMaterialInstance` _procmesh 2 (`self.VerticalProfileMaterial`) "None"))
      (`SSPVolume.UpdateSSPLineTexture` (`self.SSPVolume`) _returnvalue_2 (`local.VerticalProfileSamples`) (`local.VerticalProfileTop`) (`local.VerticalProfileBottom`))
      (`PrimitiveComponent.SetMaterial` _procmesh 0 "/Game/Ocean/M_VerticalProfileEnds.M_VerticalProfileEnds")
      (`PrimitiveComponent.SetMaterial` _procmesh 1 "/Game/Ocean/M_VerticalProfileEnds.M_VerticalProfileEnds"))))

(fn `HandleHYCOMDone`
  (bind _bathymetryreader (`self.BathymetryReader`))
  (bind _soundspeed (`Bathymetry.GetHexSoundSpeed` _bathymetryreader))
  (if (`KismetArrayLibrary.Array_IsEmpty` _soundspeed)
    ;[1 1 1] Handle hycom error with default to Munk profile
    (`KismetSystemLibrary.PrintString` "Could not get HYCOM ... defaulting to munk profile.")
    (`BellhopController.MunkProfile` (`self.Bellhop`))
    (else
      ;[1 1 1] Load the hex data from hycom
      (`|ExecutionSequence`
        (:`then_0`
          ;;[1 1 1] TODO: don't really use these copies
          (bind _output_get (set `self.HexGridX` (`Bathymetry.GetHexGridX` _bathymetryreader))))
        (:`then_1`
          (bind _output_get_2 (set `self.HexGridY` (`Bathymetry.GetHexGridY` _bathymetryreader))))
        (:`then_2`
          (bind _output_get_3 (set `self.HexDepth` (`Bathymetry.GetHexDepth` _bathymetryreader))))
        (:`then_3`
          (bind _output_get_4 (set `self.HexSSP` _soundspeed)))
        (:`then_4`
          (`BellhopController.SetHexahedralSoundSpeed` (`self.Bellhop`) _output_get _output_get_2 _output_get_3 _output_get_4)
          (`self.DrawSoundSpeedMinimum`))))))

(fn `ReadBathymetry`
  (params (North :type "Float (double-precision)") (East :type "Float (double-precision)") (South :type "Float (double-precision)") (West :type "Float (double-precision)"))
  (returns (Depth :type "Array of Float (double-precision)") (GridX :type "Array of Float (double-precision)") (GridY :type "Array of Float (double-precision)") (Success :type Boolean))
  (locals (FileErrorMessage1 :type String :default "Error: temporary hacked in file not found ... file must be at "))
  (bind (_actualnorth _actualeast _actualsouth _actualwest _gridx _gridy _depth _returnvalue) (`Bathymetry.GetEarthBathymetry` (`self.BathymetryReader`) North East South West))
  (if (`BlueprintPathsLibrary.FileExists` (`self.DepthFileName`))
    _
    (else
      _))
  (bind (_filename _returnvalue_2) (`Bathymetry.OpenTIFF` (`self.BathymetryReader`)))
  (if _returnvalue_2
    (set `self.DepthFileName` _filename)
    (if _returnvalue
      (set `self.Actual North` _actualnorth)
      (set `self.Actual East` _actualeast)
      (set `self.Actual South` _actualsouth)
      (set `self.Actual West` _actualwest)
      (return _depth _gridx _gridy true)
      (else
        (`KismetSystemLibrary.PrintString` "Error: bathymetry data not found ... check the lat/long values.")
        (return _ _ _ false)))
    (else
      (`KismetSystemLibrary.PrintString` "Error: nc file didn't open ... check the filename.")
      (return _ _ _ false))))

(fn `RunBathymetry`
  (params (North :type "Float (double-precision)") (East :type "Float (double-precision)") (South :type "Float (double-precision)") (West :type "Float (double-precision)"))
  ;[1 1 1] Load the bathymetry data and display it. This is the main thing to call.
  (`Bathymetry.SetOrigin` (`self.BathymetryReader`) South West)
  (bind (_depth _gridx _gridy _success) (`self.ReadBathymetry` North East South West))
  (if _success
    (bind _success_2 (`self.SetBathymetry` _depth _gridx _gridy))
    (if _success_2
      (`KismetSystemLibrary.PrintString` "Set Bottom OK")
      (`self.ShowBathymetry`)
      ;[1 1 1] Let the level blueprint know the bottom is loaded.
      (`self.BottomUpdated` (`.MaxValue` (`KismetMathLibrary.MaxOfFloatArray` _depth)) (`.MinValue` (`KismetMathLibrary.MinOfFloatArray` _depth)))
      (else
        (`KismetSystemLibrary.PrintString` "Error Setting Bottom")))
    (else
      (`KismetSystemLibrary.PrintString` "Error in BP_Ocean ... check the log"))))

(fn `SetBathymetry`
  (params (Depth :type "Array of Float (double-precision)") (GridX :type "Array of Float (double-precision)") (GridY :type "Array of Float (double-precision)") (O3D :type Boolean :default true))
  (returns (Success :type Boolean))
  (bind _returnvalue (`Bottom.UpdateBottom` (`self.Bottom`) Depth GridX GridY O3D))
  (return _returnvalue))

(fn `ShowBathymetry`
  (bind _bottom (`self.Bottom`))
  ;[1 1 1] The bathymetry vertices are calculated in bellhop, but use the grid mesh welded order. UV is used to map the bottom color.
  (`self.ClearBathymetry`)
  (bind _returnvalue (`Bottom.GetNPointsX` _bottom))
  (bind _returnvalue_2 (`Bottom.GetNPointsY` _bottom))
  (bind _returnvalue_3 (`Bottom.GetBottomMeshVertices` _bottom))
  (bind _returnvalue_4 (`Bottom.GetHeightMapUV` _bottom))
  (bind _triangles (`KismetProceduralMeshLibrary.CreateGridMeshWelded` _returnvalue _returnvalue_2))
  (`ProceduralMeshComponent.CreateMeshSection_LinearColor` :`self` (`self.BottomMesh`) :`Vertices` _returnvalue_3 :`Triangles` _triangles :`UV0` _returnvalue_4)
  (`PrimitiveComponent.SetMaterial` (`self.BottomMesh`) 0 (`self.M_Bottom`)))

(fn `ShowSurface`
  (locals (Vertices :type "Array of Vector Structure") (ShiftForZFighting :type "Vector Structure" :default (0.0 0.0 1.0)))
  (bind _vertices (`local.Vertices`))
  (bind _vertices_2 (`local.Vertices`))
  (bind _bathymetryreader (`self.BathymetryReader`))
  (`|ExecutionSequence`
    (:`then_0`
      ;[1 1 1] Construct the vertices
      (`KismetArrayLibrary.Array_Add` _vertices (`Bathymetry.LatLongToPosition` _bathymetryreader (`self.Actual North`) (`self.Actual East`)))
      (`KismetArrayLibrary.Array_Add` _vertices (`Bathymetry.LatLongToPosition` _bathymetryreader (`self.Actual South`) (`self.Actual East`)))
      (`KismetArrayLibrary.Array_Add` _vertices (`Bathymetry.LatLongToPosition` _bathymetryreader (`self.Actual South`) (`self.Actual West`)))
      (`KismetArrayLibrary.Array_Add` _vertices (`Bathymetry.LatLongToPosition` _bathymetryreader (`self.Actual North`) (`self.Actual West`))))
    (:`then_1`
      ;[1 1 1] Normal up view
      (bind (_triangles _vertices_3 _uvs) (`KismetProceduralMeshLibrary.CreateGridMeshSplit` 2 2))
      (`ProceduralMeshComponent.ClearAllMeshSections` (`self.SurfaceMesh`))
      (`ProceduralMeshComponent.CreateMeshSection_LinearColor` :`self` (`self.SurfaceMesh`) :`Vertices` (`local.Vertices`) :`Triangles` _triangles :`UV0` _uvs)
      (`PrimitiveComponent.SetMaterial` (`self.SurfaceMesh`) 0 (`self.SurfaceMaterial`)))
    (:`then_2`
      ;[1 1 1] Normal down view
      (bind (_triangles_2 _vertices_4 _uvs_2) (`KismetProceduralMeshLibrary.CreateGridMeshSplit` 2 2))
      (`KismetArrayLibrary.Array_Swap` _vertices_2 3 4)
      (`KismetArrayLibrary.Array_Swap` _vertices_2 1 2)
      (for (_array_element _array_index) _vertices_2
        (`KismetArrayLibrary.Array_Set` (`local.Vertices`) _array_index (- _array_element (`local.ShiftForZFighting`))))
      (`ProceduralMeshComponent.CreateMeshSection_LinearColor` :`self` (`self.SurfaceMesh`) :`SectionIndex` 1 :`Vertices` (`local.Vertices`) :`Triangles` _triangles_2 :`UV0` _uvs_2)
      (`PrimitiveComponent.SetMaterial` (`self.SurfaceMesh`) 1 (`self.SurfaceMaterialUp`)))))

(fn `UpdateGlobalBounds`
  (bind _asgi_persistent_variables (cast `/Game/Assets/GI_PersistentVariables` (`GameplayStatics.GetGameInstance`)))
  (bind _output_get (set `self.BottomBoundary` (`/Game/Assets/GI_PersistentVariables.OceanRange` _asgi_persistent_variables)))
  (if (`.IsDirty_11_26210519431F0AEE5E1B72AB12C245B6` (break `/Game/Ocean/S_OceanBounds` _output_get))
    (`KismetSystemLibrary.PrintString` "Ocean range marked as ok")
    (else
      (`KismetSystemLibrary.PrintString` "Ocean range not set. Creating default around San Diego.")
      (set `self.BottomBoundary` (`self.NESeamount`)))))

(fn `UserConstructionScript`)