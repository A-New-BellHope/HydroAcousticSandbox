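; Free-flying player character for the sandbox, with mouse-and-axis look, six-direction movement and a visible cursor.
; Forward follows camera pitch and yaw, with strafe and vertical axes alongside; each input is smoothed by FInterpTo before AddMovementInput.
; Holding Accelerate raises the shared speed multiplier on movement input.
; The RevealRays action calls StartReveal on every FollowRays actor in the level, printing a message if none exist.
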(event `InputAxis|TurnLeft/Right`
  (params (AxisValue :type "Float (single-precision)"))
  ;[0.05882 0.05882 0.05882 1 30] Rotation Controls
  (`self.AddControllerYawInput` AxisValue))

(event `InputAction|RevealRays`
  (params (Key :type "Key Structure"))
  (:`Pressed`
    (`self.RevealRays`)))

(event `self.ReceiveBeginPlay`
  ;[0.05882 0.05882 0.05882 1 30] Show mouse cursor
  (set `PlayerController.bShowMouseCursor` true (`GameplayStatics.GetPlayerController` 0))
  (bind _returnvalue (`GameplayStatics.GetActorOfClass` "/Game/Assets/Sandbox/BP_Globals.BP_Globals_C"))
  (set `self.Globals` _returnvalue))

(event `InputAxis|LookUp/Down`
  (params (AxisValue :type "Float (single-precision)"))
  ;[0.05882 0.05882 0.05882 1 30] Rotation Controls
  (`self.AddControllerPitchInput` AxisValue))

(event `InputAxis|MoveForward/Backward`
  (params (AxisValue :type "Float (single-precision)"))
  (bind (_returnvalue_roll _returnvalue_pitch _returnvalue_yaw) (`KismetMathLibrary.BreakRotator` (`self.GetControlRotation`)))
  ;[0.05729 0.05729 0.05729 1 30] Movement Controls
  (bind _output_get (set `self.CurrentForward` (`KismetMathLibrary.FInterpTo` (`self.CurrentForward`) AxisValue (`GameplayStatics.GetWorldDeltaSeconds`) 6.0)))
  (`self.AddMovementInput` (`KismetMathLibrary.GetForwardVector` (`KismetMathLibrary.MakeRotator` 0.0 _returnvalue_pitch _returnvalue_yaw)) (* _output_get (`self.SpeedMultiplier`))))

(event `InputAxis|StrafeLeft/Right`
  (params (AxisValue :type "Float (single-precision)"))
  (bind (_returnvalue_roll _returnvalue_pitch _returnvalue_yaw) (`KismetMathLibrary.BreakRotator` (`self.GetControlRotation`)))
  ;[0.05729 0.05729 0.05729 1 30] Movement Controls
  (bind _output_get (set `self.CurrentStrafe` (`KismetMathLibrary.FInterpTo` (`self.CurrentStrafe`) AxisValue (`GameplayStatics.GetWorldDeltaSeconds`) 6.0)))
  (`self.AddMovementInput` (`KismetMathLibrary.GetRightVector` (`KismetMathLibrary.MakeRotator` _returnvalue_roll 0.0 _returnvalue_yaw)) (* _output_get (`self.SpeedMultiplier`))))

(event `InputAxis|MoveUp/Down`
  (params (AxisValue :type "Float (single-precision)"))
  (bind (_returnvalue_roll _returnvalue_pitch _returnvalue_yaw) (`KismetMathLibrary.BreakRotator` (`self.GetControlRotation`)))
  ;[0.05729 0.05729 0.05729 1 30] Movement Controls
  (bind _output_get (set `self.CurrentUpDown` (`KismetMathLibrary.FInterpTo` (`self.CurrentUpDown`) AxisValue (`GameplayStatics.GetWorldDeltaSeconds`) 6.0)))
  (`self.AddMovementInput` (`KismetMathLibrary.GetUpVector` (`KismetMathLibrary.MakeRotator` 0.0 0.0 _returnvalue_yaw)) (* _output_get (`self.SpeedMultiplier`))))

(event `InputAction|Accelerate`
  (params (Key :type "Key Structure"))
  ;[0.05729 0.05729 0.05729 1 30] Movement Controls
  (:`Pressed`
    (set `self.SpeedMultiplier` 20.0))
  (:`Released`
    (set `self.SpeedMultiplier` 1.0)))

(fn `RevealRays`
  (locals (AllRays :type "Array of FollowRays Object Reference"))
  (bind _allrays (`local.AllRays`))
  (bind _outactors (`GameplayStatics.GetAllActorsOfClass` "/Script/bellhop.FollowRays"))
  (set `local.AllRays` _outactors)
  (if (`KismetArrayLibrary.Array_IsEmpty` _allrays)
    (`KismetSystemLibrary.PrintString` "No Rays in level")
    (else
      (for _array_element _allrays
        (`FollowRays.StartReveal` _array_element)))))

(fn `UserConstructionScript`)