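; BP_SoundMover is an actor that positions itself at a sound source location read from Bellhop.
; When the bound sound-source-placed event fires, it fetches the location by SourceID, converts Z, moves its root there and enables player input.
; The MoveSoundSourceMode input and MoveActorOutofSight event toggle it between that position and a point far below the world, a stopgap for hiding it when unused.
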(event `self.ReceiveBeginPlay`
  (add `self.SoundSourcePlaced` (delegate `MoveToSoundsource`)))

(event `MoveToSoundsource`
  (bind _returnvalue (`BellhopController.GetSourceLocation` (`self.Bellhop`) (`self.Source ID`)))
  (bind _result (`/Engine/EditorBlueprintResources/StandardMacros.NegateFloat` (.z _returnvalue))
    (:`  `
      (set `self.SoundSourcePos` (`KismetMathLibrary.MakeVector` (.x _returnvalue) (.y _returnvalue) _result))
      (`SceneComponent.K2_SetWorldLocation` (`self.DefaultSceneRoot`) (`self.SoundSourcePos`) false false)
      (`self.EnableInput` (`GameplayStatics.GetPlayerController` 0)))))

(event `InputAction|MoveSoundSourceMode`
  (params (Key :type "Key Structure"))
  (:`Pressed`
    ;[0.1667 0.1667 0.1667] Temporary solution:  Move far away when not using
    (if (`self.MoveOutOfSight`) :!label _label
      (set `self.MoveOutOfSight` false)
      (`SceneComponent.K2_SetWorldLocation` (`self.DefaultSceneRoot`) (0.0 0.0 -10000000.0) false false)
      (else
        (set `self.MoveOutOfSight` true)
        (`SceneComponent.K2_SetWorldLocation` (`self.DefaultSceneRoot`) (`self.SoundSourcePos`) false false)))))

(event `MoveActorOutofSight`
  ;[0.1667 0.1667 0.1667] Temporary solution:  Move far away when not using
  (goto _label))

(fn `UserConstructionScript`)