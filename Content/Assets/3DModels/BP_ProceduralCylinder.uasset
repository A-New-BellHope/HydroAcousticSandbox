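; Procedural cylinder actor that builds its mesh at BeginPlay from Radius, Height and Sides, with the base at local Z=0.
; GenerateCylinder clears the ProcMesh and writes three sections: top cap, bottom cap and side wall, reusing shared vertex, triangle, normal and UV arrays.
; Caps are triangle fans with planar UVs, while the wall has smooth radial normals and a duplicated seam for UV wrapping.
; SetHeight, SetRadius and SetSides each regenerate the whole mesh.
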(event `self.ReceiveBeginPlay`
  (`self.GenerateCylinder`))

(fn `GenerateCylinder`
  (locals (Vertices :type "Array of Vector Structure") (Triangles :type "Array of Integer") (Normals :type "Array of Vector Structure") (UVs :type "Array of Vector2D Structure") (TWO_PI :type "Float (double-precision)"))
  (bind _triangles (`local.Triangles`))
  (bind _triangles_2 (`local.Triangles`))
  (bind _sides (`self.Sides`))
  (bind _sides_2 (`self.Sides`))
  (set `local.TWO_PI` (* (`KismetMathLibrary.Acos` -1.0) 2.0))
  (`ProceduralMeshComponent.ClearAllMeshSections` (`self.ProcMesh`))
  (`|ExecutionSequence`
    (:`then_0`
      ;[1 1 1] Top
      (`KismetArrayLibrary.Array_Clear` (`local.Vertices`))
      (`KismetArrayLibrary.Array_Clear` (`local.Triangles`))
      (`KismetArrayLibrary.Array_Clear` (`local.Normals`))
      (`KismetArrayLibrary.Array_Clear` (`local.UVs`))
      (`KismetArrayLibrary.Array_Add` (`local.Vertices`) (`KismetMathLibrary.MakeVector` 0.0 0.0 (`self.Height`)))
      (`KismetArrayLibrary.Array_Add` (`local.Normals`) (0.0 0.0 1.0))
      (`KismetArrayLibrary.Array_Add` (`local.UVs`) (0.5 0.5))
      (for _index (range (`self.Sides`))
        (bind _returnvalue (* _index (`local.TWO_PI`) (`KismetMathLibrary.SafeDivide` 1.0 (`KismetMathLibrary.Conv_IntToDouble` (`self.Sides`)))))
        (bind _returnvalue_2 (`KismetMathLibrary.Sin` _returnvalue))
        (bind _returnvalue_3 (`KismetMathLibrary.Cos` _returnvalue))
        (`KismetArrayLibrary.Array_Add` (`local.Vertices`) (`KismetMathLibrary.MakeVector` (* _returnvalue_2 (`self.Radius`)) (* _returnvalue_3 (`self.Radius`)) (`self.Height`)))
        (`KismetArrayLibrary.Array_Add` (`local.UVs`) (`KismetMathLibrary.MakeVector2D` (/ (+ _returnvalue_3 1.0) 2.0) (/ (+ _returnvalue_2 1.0) 2.0)))
        (`KismetArrayLibrary.Array_Add` (`local.Normals`) (0.0 0.0 1.0)))
      (for _index_2 (range 1 (+ _sides 1))
        (`KismetArrayLibrary.Array_Add` (`local.Triangles`))
        (`KismetArrayLibrary.Array_Add` (`local.Triangles`) _index_2)
        (`KismetArrayLibrary.Array_Add` (`local.Triangles`) (+ (mod _index_2 _sides) 1)))
      (`ProceduralMeshComponent.CreateMeshSection_LinearColor` :`self` (`self.ProcMesh`) :`Vertices` (`local.Vertices`) :`Triangles` (`local.Triangles`) :`Normals` (`local.Normals`) :`UV0` (`local.UVs`)))
    (:`then_1`
      ;[1 1 1] Bottom
      (`KismetArrayLibrary.Array_Clear` (`local.Vertices`))
      (`KismetArrayLibrary.Array_Clear` (`local.Triangles`))
      (`KismetArrayLibrary.Array_Clear` (`local.Normals`))
      (`KismetArrayLibrary.Array_Clear` (`local.UVs`))
      (`KismetArrayLibrary.Array_Add` (`local.Vertices`))
      (`KismetArrayLibrary.Array_Add` (`local.Normals`) (0.0 0.0 -1.0))
      (`KismetArrayLibrary.Array_Add` (`local.UVs`) (0.5 0.5))
      (for _index_3 (range (`self.Sides`))
        (bind _returnvalue_4 (* _index_3 (`local.TWO_PI`) (`KismetMathLibrary.SafeDivide` 1.0 (`KismetMathLibrary.Conv_IntToDouble` (`self.Sides`)))))
        (bind _returnvalue_5 (`KismetMathLibrary.Sin` _returnvalue_4))
        (bind _returnvalue_6 (`KismetMathLibrary.Cos` _returnvalue_4))
        (`KismetArrayLibrary.Array_Add` (`local.Vertices`) (`KismetMathLibrary.MakeVector` (* _returnvalue_5 (`self.Radius`)) (* _returnvalue_6 (`self.Radius`))))
        (`KismetArrayLibrary.Array_Add` (`local.UVs`) (`KismetMathLibrary.MakeVector2D` (/ (+ _returnvalue_6 1.0) 2.0) (/ (+ _returnvalue_5 1.0) 2.0)))
        (`KismetArrayLibrary.Array_Add` (`local.Normals`) (0.0 0.0 -1.0)))
      (for _index_4 (range 1 (+ _sides_2 1))
        (`KismetArrayLibrary.Array_Add` (`local.Triangles`))
        (`KismetArrayLibrary.Array_Add` (`local.Triangles`) (+ (mod _index_4 _sides_2) 1))
        (`KismetArrayLibrary.Array_Add` (`local.Triangles`) _index_4))
      (`ProceduralMeshComponent.CreateMeshSection_LinearColor` :`self` (`self.ProcMesh`) :`SectionIndex` 1 :`Vertices` (`local.Vertices`) :`Triangles` (`local.Triangles`) :`Normals` (`local.Normals`) :`UV0` (`local.UVs`)))
    (:`then_2`
      ;[1 1 1] Side
      (`KismetArrayLibrary.Array_Clear` (`local.Vertices`))
      (`KismetArrayLibrary.Array_Clear` (`local.Triangles`))
      (`KismetArrayLibrary.Array_Clear` (`local.Normals`))
      (`KismetArrayLibrary.Array_Clear` (`local.UVs`))
      (for _index_5 (range (+ (`self.Sides`) 1))
        (bind _returnvalue_7 (* _index_5 (`local.TWO_PI`) (`KismetMathLibrary.SafeDivide` 1.0 (`KismetMathLibrary.Conv_IntToDouble` (`self.Sides`)))))
        (bind _returnvalue_8 (`KismetMathLibrary.Cos` _returnvalue_7))
        (bind _returnvalue_9 (* _returnvalue_8 (`self.Radius`)))
        (bind _returnvalue_10 (`KismetMathLibrary.Sin` _returnvalue_7))
        (bind _returnvalue_11 (* _returnvalue_10 (`self.Radius`)))
        (`KismetArrayLibrary.Array_Add` (`local.Vertices`) (`KismetMathLibrary.MakeVector` _returnvalue_9 _returnvalue_11))
        (`KismetArrayLibrary.Array_Add` (`local.Normals`) (`KismetMathLibrary.MakeVector` _returnvalue_8 _returnvalue_10))
        (bind _returnvalue_12 (`KismetMathLibrary.SafeDivide` (`KismetMathLibrary.Conv_IntToDouble` _index_5) (`KismetMathLibrary.Conv_IntToDouble` (`self.Sides`))))
        (`KismetArrayLibrary.Array_Add` (`local.UVs`) (`KismetMathLibrary.MakeVector2D` _returnvalue_12 1.0))
        (`KismetArrayLibrary.Array_Add` (`local.Vertices`) (`KismetMathLibrary.MakeVector` _returnvalue_9 _returnvalue_11 (`self.Height`)))
        (`KismetArrayLibrary.Array_Add` (`local.Normals`) (`KismetMathLibrary.MakeVector` _returnvalue_8 _returnvalue_10))
        (`KismetArrayLibrary.Array_Add` (`local.UVs`) (`KismetMathLibrary.MakeVector2D` _returnvalue_12)))
      (for _index_6 (range (`self.Sides`))
        (bind _returnvalue_13 (* _index_6 2))
        (`KismetArrayLibrary.Array_Add` _triangles_2 _returnvalue_13)
        (`KismetArrayLibrary.Array_Add` _triangles_2 (+ _returnvalue_13 1))
        (bind _returnvalue_14 (* (+ _index_6 1) 2))
        (bind _returnvalue_15 (+ _returnvalue_14 1))
        (`KismetArrayLibrary.Array_Add` _triangles_2 _returnvalue_15)
        (`KismetArrayLibrary.Array_Add` _triangles _returnvalue_13)
        (`KismetArrayLibrary.Array_Add` _triangles _returnvalue_15)
        (`KismetArrayLibrary.Array_Add` _triangles _returnvalue_14))
      (`ProceduralMeshComponent.CreateMeshSection_LinearColor` :`self` (`self.ProcMesh`) :`SectionIndex` 2 :`Vertices` (`local.Vertices`) :`Triangles` (`local.Triangles`) :`Normals` (`local.Normals`) :`UV0` (`local.UVs`)))))

(fn `SetHeight`
  (params (Height :type "Float (double-precision)"))
  (set `self.Height` Height)
  (`self.GenerateCylinder`))

(fn `SetRadius`
  (params (Radius :type "Float (double-precision)"))
  (set `self.Radius` Radius)
  (`self.GenerateCylinder`))

(fn `SetSides`
  (params (Sides :type Integer))
  (set `self.Sides` Sides)
  (`self.GenerateCylinder`))

(fn `UserConstructionScript`)