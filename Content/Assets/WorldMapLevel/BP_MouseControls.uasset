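; BP_MouseControls handles mouse input on the world map level, for picking a geographic area and zooming the camera.
; Right-click press traces under the cursor, converting the impact normal and hit actor's rotation into latitude and longitude, as on a globe.
; Release builds a bounding box around that point and writes it to GI_PersistentVariables' BottomRange.
; The mouse wheel zooms LevelCamera by stepping its clamped field of view.
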(event `self.ReceiveBeginPlay`
  (`self.EnableInput` (`GameplayStatics.GetPlayerController` 0))
  (`KismetSystemLibrary.Delay` 0.2)
  (bind _foundwidgets (`WidgetBlueprintLibrary.GetAllWidgetsOfClass` "/Game/Assets/WorldMapLevel/WB_LevelSelect.WB_LevelSelect_C"))
  (for _array_element _foundwidgets
    (set `self.Widget` _array_element)))

(event `Key|RightMouseButton`
  (params (Key :type "Key Structure"))
  (bind (_worldlocation _worlddirection) (`PlayerController.DeprojectMousePositionToWorld` (`GameplayStatics.GetPlayerController` 0)))
  (:`Pressed`
    (bind _outhit (`KismetSystemLibrary.LineTraceSingle` _worldlocation (+ _worldlocation (* _worlddirection 100000.0)) "TraceTypeQuery2"))
    (bind (_bblockinghit _binitialoverlap _time _distance _location _impactpoint _normal _impactnormal _physmat _hitactor) (`GameplayStatics.BreakHitResult` _outhit))
    (bind (_latitude _longitude) (`self.GetLatLongCoordinates` _impactnormal _hitactor))
    (set `self.MousePointLongitude` _longitude)
    (set `self.MousePointLatitude` _latitude))
  (:`Released`
    (`self.CreateBoundingBox` 1.0 (`self.MousePointLatitude`) (`self.MousePointLongitude`))))

(event `Key|MouseScrollUp`
  (params (Key :type "Key Structure"))
  (bind _cameracomponent (`CameraActor.CameraComponent` (`self.LevelCamera`)))
  (:`Pressed`
    (`CameraComponent.SetFieldOfView` _cameracomponent (`KismetMathLibrary.FClamp` (- (`CameraComponent.FieldOfView` _cameracomponent) 5.0) 30.0 50.0))))

(event `Key|MouseScrollDown`
  (params (Key :type "Key Structure"))
  (bind _cameracomponent (`CameraActor.CameraComponent` (`self.LevelCamera`)))
  (:`Pressed`
    (`CameraComponent.SetFieldOfView` _cameracomponent (`KismetMathLibrary.FClamp` (+ (`CameraComponent.FieldOfView` _cameracomponent) 5.0) 30.0 50.0))))

(fn `CreateBoundingBox`
  (params (BoxSize :type "Float (double-precision)") (Latitude :type "Float (double-precision)") (Longitude :type "Float (double-precision)"))
  (`KismetSystemLibrary.PrintString` (`KismetStringLibrary.Conv_DoubleToString` Latitude))
  (`KismetSystemLibrary.PrintString` (`KismetStringLibrary.Conv_DoubleToString` Longitude))
  (set `self.NorthCoordinate` (+ BoxSize Latitude))
  (set `self.SouthCoordinate` (- Latitude BoxSize))
  (set `self.EastCoordinate` (+ BoxSize Longitude))
  (set `self.WestCoordinate` (- Longitude BoxSize))
  ;[1 1 1] Synchronize the persistent variables
  (bind _asgi_persistent_variables (cast `/Game/Assets/GI_PersistentVariables` (`GameplayStatics.GetGameInstance`))
    (:`then`
      (bind _output_get (set `self.PersistentVariables` _asgi_persistent_variables))
      (set `/Game/Assets/GI_PersistentVariables.BottomRange` (make `/Game/Bottom/S_BottomBoundary` (`self.NorthCoordinate`) (`self.EastCoordinate`) (`self.SouthCoordinate`) (`self.WestCoordinate`) true) _output_get))
    (:`CastFailed`
      (`KismetSystemLibrary.PrintString` "Error: failed to find GI_PersitentVariable. Check that the main Game Instance is a GI_PersistentVariable ... unknown results to follow" true true (struct :`R` 1.0 :`B` 0.187721 :`A` 1.0) 12.0))))

(fn `GetLatLongCoordinates`
  (params (InVector :type "Vector Structure") (HitActor :type "Actor Object Reference"))
  (returns (Latitude :type "Float (double-precision)") (Longitude :type "Float (double-precision)"))
  (bind _x (.x InVector))
  (bind _y (.y InVector))
  (return (+ (`KismetMathLibrary.DegAtan2` (.z InVector) (`KismetMathLibrary.Sqrt` (+ (`KismetMathLibrary.Square` _x) (`KismetMathLibrary.Square` _y)))) (.pitch (`self.K2_GetActorRotation` HitActor))) (+ (`KismetMathLibrary.DegAtan2` _x _y) (.yaw (`self.K2_GetActorRotation` HitActor)))))

(fn `UserConstructionScript`)