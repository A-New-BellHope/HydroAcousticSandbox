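; Rotating globe actor for the world map level that spins with mouse dragging and keeps turning with inertia.
; Clicking the globe starts a drag, during which Tick accumulates input axis values into yaw and pitch velocities until release.
; Each tick applies those velocities as world rotation to the root, decaying them by a frame-rate-dependent per-frame damping factor.
; Pressing R clears the motion and restores the rotation saved at BeginPlay.
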(event `self.ReceiveBeginPlay`
  (set `self.StartRotation` (`self.K2_GetActorRotation`)))

(event `self.Globe.OnClicked`
  (params (TouchedComponent :type "PrimitiveComponent Object Reference") (ButtonPressed :type "Key Structure"))
  (set `self.StartDragging` true))

(event `self.ReceiveTick`
  (params (DeltaSeconds :type "Float (single-precision)"))
  (`self.HandleMouseDrag` DeltaSeconds)
  (`self.HandleGlobeRotation` DeltaSeconds))

(event `self.Globe.OnReleased`
  (params (TouchedComponent :type "PrimitiveComponent Object Reference") (ButtonReleased :type "Key Structure"))
  (set `self.StartDragging` false))

(event `Key|R`
  (params (Key :type "Key Structure"))
  (:`Pressed`
    (`self.ResetRotation`)))

(fn `HandleGlobeRotation`
  (params (`Delta Seconds` :type "Float (double-precision)"))
  (bind _pitchrotatevelocity (`self.PitchRotateVelocity`))
  (bind _yawrotatevelocity (`self.YawRotateVelocity`))
  (`SceneComponent.K2_AddWorldRotation` (`self.DefaultSceneRoot`) (`KismetMathLibrary.MakeRotator` 0.0 (* (`self.PitchRotateVelocity`) `Delta Seconds`) (* `Delta Seconds` (`self.YawRotateVelocity`))) false false)
  (if (or (< _yawrotatevelocity -0.1) (> _yawrotatevelocity 0.1) (< _pitchrotatevelocity -0.1) (> _pitchrotatevelocity 0.1))
    (set `self.YawRotateVelocity` (* (`self.YawRotateVelocity`) 0.95))
    (set `self.DragSumX` (* (`self.DragSumX`) 0.95))
    (set `self.PitchRotateVelocity` (* (`self.PitchRotateVelocity`) 0.95))
    (set `self.DragSumY` (* (`self.DragSumY`) 0.95))))

(fn `HandleMouseDrag`
  (params (`Delta Seconds` :type "Float (double-precision)"))
  (if (`self.StartDragging`)
    (bind _output_get (set `self.DragSumX` (- (`self.DragSumX`) (`self.GetInputAxisKeyValue`))))
    (set `self.YawRotateVelocity` (+ (`self.YawRotateVelocity`) (* (* _output_get `Delta Seconds`) 60.0)))
    (bind _output_get_2 (set `self.DragSumY` (- (`self.DragSumY`) (`self.GetInputAxisKeyValue`))))
    (set `self.PitchRotateVelocity` (+ (`self.PitchRotateVelocity`) (* (* _output_get_2 `Delta Seconds`) 60.0)))
    (else
      (set `self.DragSumX` 0.0)
      (set `self.DragSumY` 0.0))))

(fn `ResetRotation`
  (returns (Output :type Boolean))
  (`|ExecutionSequence`
    (:`then_0`
      (set `self.DragSumY` 0.0))
    (:`then_1`
      (set `self.DragSumX` 0.0))
    (:`then_2`
      (set `self.PitchRotateVelocity` 0.0))
    (:`then_3`
      (set `self.YawRotateVelocity` 0.0)
      (bind _returnvalue (`self.K2_SetActorRotation` (`self.StartRotation`)))
      (return _returnvalue))))

(fn `UserConstructionScript`)