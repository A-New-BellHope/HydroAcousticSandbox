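; World map marker actor that draws a latitude/longitude selection rectangle on the rotating globe.
; InitializeSquare anchors the first corner at the last picked point and creates a procedural quad.
; While a marker is started and the mouse moves, Tick updates that quad and writes the sorted bounds to OceanRange in the persistent game instance.
; Corners come from the globe's LatLongToLocation in actor-local space; the maximum-size input is unused.
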(event `self.ReceiveBeginPlay`
  (bind _asgi_persistent_variables (cast `/Game/Assets/GI_PersistentVariables` (`GameplayStatics.GetGameInstance`))
    (:`then`
      (set `self.PersistentVariables` _asgi_persistent_variables))
    (:`CastFailed`
      (`KismetSystemLibrary.PrintString` "Error: failed to find GI_PersitentVariable. Check that the main Game Instance is a GI_PersistentVariable ... unknown results to follow" true true (struct :`R` 1.0 :`B` 0.187721 :`A` 1.0) 12.0)))
  ;[1 1 1] For the latlong to point map
  (bind _returnvalue (`GameplayStatics.GetActorOfClass` "/Game/Assets/WorldMapLevel/BP_RotatingGlobe.BP_RotatingGlobe_C"))
  (set `self.RotatingGlobe` _returnvalue))

(event `self.ReceiveTick`
  (params (DeltaSeconds :type "Float (single-precision)"))
  (bind (_worldselect_lastlatitude _worldselect_lastlongitude _worldselect_location _worldselect_normal _worldselect_actor _worldselect_mousemoved _worldselect_markerstarted) (break `/Game/Assets/WorldMapLevel/S_WorldSelect` (`/Game/Assets/GI_PersistentVariables.WorldSelect` (`self.PersistentVariables`))))
  (if (and _worldselect_mousemoved _worldselect_markerstarted)
    (`self.UpdateSquare` 100000.0)))

(fn `InitializeSquare`
  (locals (QuadTriangles :type "Array of Integer"))
  (bind (_worldselect_lastlatitude _worldselect_lastlongitude _worldselect_location _worldselect_normal) (break `/Game/Assets/WorldMapLevel/S_WorldSelect` (`/Game/Assets/GI_PersistentVariables.WorldSelect` (`self.PersistentVariables`))))
  (`ProceduralMeshComponent.ClearAllMeshSections` (`self.SelectedRegion`))
  (bind _output_get (set `self.Latitude1` _worldselect_lastlatitude))
  (bind _output_get_2 (set `self.Longitude1` _worldselect_lastlongitude))
  (bind _output_get_3 (set `self.StartNormal` _worldselect_normal))
  (bind _vertices (`self.RectFromPointNormal` _output_get _output_get_2 _output_get _output_get_2 _output_get_3))
  (`ProceduralMeshComponent.CreateMeshSection_LinearColor` :`self` (`self.SelectedRegion`) :`Vertices` _vertices :`Triangles` (`local.QuadTriangles`))
  (`PrimitiveComponent.SetMaterial` (`self.SelectedRegion`) 0 "/Game/Assets/WorldMapLevel/M_WorldMarker.M_WorldMarker"))

(fn `RectFromPointNormal`
  (params (Latitude1 :type "Float (double-precision)") (Longitude1 :type "Float (double-precision)") (Latitude2 :type "Float (double-precision)") (Longitude2 :type "Float (double-precision)") (Normal :type "Vector Structure") (MaxDiagonal :type "Float (double-precision)"))
  (returns (Vertices :type "Array of Vector Structure"))
  (locals (VertexOut :type "Array of Vector Structure") (n :type "Vector Structure") (Start :type "Vector Structure") (zero :type "Vector Structure") (StartLatitude :type "Float (double-precision)" :default 0.0) (StartLongitude :type "Float (double-precision)" :default 0.0) (CornerLatitude :type "Float (double-precision)" :default 0.0) (CornerLongitude :type "Float (double-precision)" :default 0.0))
  ;[1 1 1] Initialize
  (set `local.n` Normal)
  (set `local.StartLatitude` Latitude1)
  (set `local.StartLongitude` Longitude1)
  (set `local.CornerLatitude` Latitude2)
  (set `local.CornerLongitude` Longitude2)
  (`|ExecutionSequence`
    (:`then_0`
      ;[1 1 1] Corner 1
      (bind _location (`/Game/Assets/WorldMapLevel/BP_RotatingGlobe.LatLongToLocation` (`self.RotatingGlobe`) (`local.StartLatitude`) (`local.StartLongitude`)))
      (`KismetArrayLibrary.Array_Add` (`local.VertexOut`) (`KismetMathLibrary.InverseTransformLocation` (`self.GetTransform`) _location)))
    (:`then_1`
      ;[1 1 1] Corner 2
      (bind _location_2 (`/Game/Assets/WorldMapLevel/BP_RotatingGlobe.LatLongToLocation` (`self.RotatingGlobe`) (`local.StartLatitude`) (`local.CornerLongitude`)))
      (`KismetArrayLibrary.Array_Add` (`local.VertexOut`) (`KismetMathLibrary.InverseTransformLocation` (`self.GetTransform`) _location_2)))
    (:`then_2`
      ;[1 1 1] Corner 3
      (bind _location_3 (`/Game/Assets/WorldMapLevel/BP_RotatingGlobe.LatLongToLocation` (`self.RotatingGlobe`) (`local.CornerLatitude`) (`local.CornerLongitude`)))
      (`KismetArrayLibrary.Array_Add` (`local.VertexOut`) (`KismetMathLibrary.InverseTransformLocation` (`self.GetTransform`) _location_3)))
    (:`then_3`
      ;[1 1 1] Corner 4
      (bind _location_4 (`/Game/Assets/WorldMapLevel/BP_RotatingGlobe.LatLongToLocation` (`self.RotatingGlobe`) (`local.CornerLatitude`) (`local.StartLongitude`)))
      (`KismetArrayLibrary.Array_Add` (`local.VertexOut`) (`KismetMathLibrary.InverseTransformLocation` (`self.GetTransform`) _location_4))
      (return (`local.VertexOut`)))))

(fn `UpdateSquare`
  (params (MaxSize :type "Float (double-precision)" :default 1.0))
  (bind _latitude1 (`self.Latitude1`))
  (bind _longitude1 (`self.Longitude1`))
  (bind (_worldselect_lastlatitude _worldselect_lastlongitude _worldselect_location _worldselect_normal) (break `/Game/Assets/WorldMapLevel/S_WorldSelect` (`/Game/Assets/GI_PersistentVariables.WorldSelect` (`self.PersistentVariables`))))
  (bind _returnvalue (`KismetMathLibrary.FMin` _latitude1 _worldselect_lastlatitude))
  (bind _returnvalue_2 (`KismetMathLibrary.FMax` _latitude1 _worldselect_lastlatitude))
  (bind _returnvalue_3 (`KismetMathLibrary.FMin` _worldselect_lastlongitude _longitude1))
  (bind _returnvalue_4 (`KismetMathLibrary.FMax` _worldselect_lastlongitude _longitude1))
  (setmembers `/Game/Ocean/S_OceanBounds` :`StructRef` (`/Game/Assets/GI_PersistentVariables.OceanRange` (`self.PersistentVariables`)) :`North` _returnvalue_2 :`East` _returnvalue_4 :`South` _returnvalue :`West` _returnvalue_3 :`IsDirty` true)
  (bind _vertices (`self.RectFromPointNormal` _returnvalue _returnvalue_3 _returnvalue_2 _returnvalue_4 _worldselect_normal MaxSize))
  (`ProceduralMeshComponent.UpdateMeshSection_LinearColor` :`self` (`self.SelectedRegion`) :`Vertices` _vertices)
  (setmembers `/Game/Assets/WorldMapLevel/S_WorldSelect` :`StructRef` (`/Game/Assets/GI_PersistentVariables.WorldSelect` (`self.PersistentVariables`)) :`MouseMoved` false))

(fn `UserConstructionScript`)