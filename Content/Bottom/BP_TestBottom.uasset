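; BP_TestBottom is a test actor that loads seafloor bathymetry for a Bellhop 3D ray simulation.
; BeginPlay spawns reader, bottom and Bellhop helpers and takes the boundary from the persistent GameInstance.
; ConstructSimulation, when that boundary is dirty, wraps its coordinates to ±180, reads depths from an nc file and updates the bottom.
; Procedural mesh display and FollowRays spawning are implemented, but their calls in RunBathymetry are disconnected.
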(event `self.ReceiveBeginPlay`
  (`|ExecutionSequence`
    (:`then_0`
      ;[1 1 1] Initialize objects or find references
      (bind _returnvalue (`|SpawnActorFromClass` "/Script/netcdfunreal.Bathymetry" (`self.Zero`) "Undefined" "MultiplyWithRoot" null null))
      (set `self.BathymetryReader` _returnvalue)
      (bind _returnvalue_2 (`|SpawnActorFromClass` "/Script/bellhop.Bottom" (`self.Zero`) "Undefined" "MultiplyWithRoot" null null))
      (set `self.Bottom` _returnvalue_2)
      (bind _returnvalue_3 (`|SpawnActorFromClass` "/Script/bellhop.BellhopController" (`self.Zero`) "Undefined" "MultiplyWithRoot" null null))
      (set `self.Bellhop` _returnvalue_3)
      (bind _asgi_persistent_variables (cast `/Game/Assets/GI_PersistentVariables` (`GameplayStatics.GetGameInstance`)))
      (set `self.BottomBoundary` (`/Game/Assets/GI_PersistentVariables.BottomRange` _asgi_persistent_variables)))
    (:`then_1`
      ;[1 1 1] Initialize bellhop in 3d
      (`BellhopController.SetupDefaults` (`self.Bellhop`) (`self.O3D`) (`self.R3D`)))))

(event `ConstructSimulation`
  (bind (_bottomboundary_north _bottomboundary_east _bottomboundary_south _bottomboundary_west) (break `/Game/Bottom/S_BottomBoundary` (`self.BottomBoundary`)))
  (bind (_bottomboundary_north_2 _bottomboundary_east_2 _bottomboundary_south_2 _bottomboundary_west_2 _bottomboundary_isdirty) (break `/Game/Bottom/S_BottomBoundary` (`self.BottomBoundary`)))
  (if _bottomboundary_isdirty
    (`|ExecutionSequence`
      (:`then_0`
        (bind _valuefix (`self.CheckRange` _bottomboundary_north))
        (set `self.VNorth` _valuefix))
      (:`then_1`
        (bind _valuefix_2 (`self.CheckRange` _bottomboundary_east))
        (set `self.VEast` _valuefix_2))
      (:`then_2`
        (bind _valuefix_3 (`self.CheckRange` _bottomboundary_south))
        (set `self.VSouth` _valuefix_3))
      (:`then_3`
        (bind _valuefix_4 (`self.CheckRange` _bottomboundary_west))
        (set `self.VWest` _valuefix_4))
      (:`then_4`
        (`self.RunBathymetry` (`self.VNorth`) (`self.VEast`) (`self.VSouth`) (`self.VWest`))))))

(fn `CheckRange`
  (params (Value :type "Float (double-precision)"))
  (returns (ValueFix :type "Float (double-precision)"))
  (locals (res :type "Float (double-precision)"))
  (bind _output_get (set `local.res` Value))
  (`|ExecutionSequence`
    (:`then_0`
      (while (< _output_get -180.0)
        (set `local.res` (+ (`local.res`) 360.0))))
    (:`then_1`
      (while (>= _output_get 180.0)
        (set `local.res` (- (`local.res`) 360.0))))
    (:`then_2`
      (return (`local.res`)))))

(fn `ClearBathymetry`
  (`ProceduralMeshComponent.ClearAllMeshSections` (`self.BottomMesh`)))

(fn `ClearRays`
  (bind _outactors (`GameplayStatics.GetAllActorsOfClass` "/Script/bellhop.FollowRays"))
  (for _array_element _outactors
    (`self.K2_DestroyActor` _array_element)))

(fn `ReadBathymetry`
  (params (North :type "Float (double-precision)") (East :type "Float (double-precision)") (South :type "Float (double-precision)") (West :type "Float (double-precision)"))
  (returns (Depth :type "Array of Float (double-precision)") (GridX :type "Array of Float (double-precision)") (GridY :type "Array of Float (double-precision)") (Success :type Boolean))
  (locals (FileErrorMessage1 :type String :default "Error: temporary hacked in file not found ... file must be at "))
  (bind _depthfilename (`self.DepthFileName`))
  (bind (_gridx _gridy _depth _returnvalue) (`Bathymetry.GetEarthBathymetry` (`self.BathymetryReader`) North East South West))
  (if (`BlueprintPathsLibrary.FileExists` _depthfilename)
    (bind _returnvalue_2 (`Bathymetry.LoadEarthFile` (`self.BathymetryReader`) _depthfilename))
    (if _returnvalue_2
      (if _returnvalue
        (return _depth _gridx _gridy true)
        (else
          (`KismetSystemLibrary.PrintString` "Error: bathymetry data not found ... check the lat/long values.")
          (return _ _ _ false)))
      (else
        (`KismetSystemLibrary.PrintString` "Error: nc file didn't open ... check the filename.")
        (return _ _ _ false)))
    (else
      (`KismetSystemLibrary.PrintString` (`KismetStringLibrary.Concat_StrStr` (`local.FileErrorMessage1`) (`self.DepthFileName`)))
      (return _ _ _ false))))

(fn `RunBathymetry`
  (params (North :type "Float (double-precision)") (East :type "Float (double-precision)") (South :type "Float (double-precision)") (West :type "Float (double-precision)"))
  ;[1 1 1] Load the bathymetry data and display it. This is the main thing to call.
  (bind (_depth _gridx _gridy) (`self.ReadBathymetry` North East South West))
  (bind _success (`self.SetBathymetry` _depth _gridx _gridy)))

(fn `SetBathymetry`
  (params (Depth :type "Array of Float (double-precision)") (GridX :type "Array of Float (double-precision)") (GridY :type "Array of Float (double-precision)") (O3D :type Boolean :default true))
  (returns (Success :type Boolean))
  (bind _returnvalue (`Bottom.UpdateBottom` (`self.Bottom`) Depth GridX GridY O3D))
  (return _returnvalue))

(fn `ShowBathymetry`
  (bind _bottom (`self.Bottom`))
  (`self.ClearBathymetry`)
  (bind _returnvalue (`Bottom.GetNPointsX` _bottom))
  (bind _returnvalue_2 (`Bottom.GetNPointsY` _bottom))
  (bind _returnvalue_3 (`Bottom.GetBottomMeshVertices` _bottom))
  (bind _returnvalue_4 (`Bottom.GetHeightMapUV` _bottom))
  (bind _triangles (`KismetProceduralMeshLibrary.CreateGridMeshWelded` _returnvalue _returnvalue_2))
  (`ProceduralMeshComponent.CreateMeshSection_LinearColor` :`self` (`self.BottomMesh`) :`Vertices` _returnvalue_3 :`Triangles` _triangles :`UV0` _returnvalue_4)
  (`PrimitiveComponent.SetMaterial` (`self.BottomMesh`) 0 (`self.M_Bottom`)))

(fn `ShowRays`
  (locals (AltitudeLow :type "Float (single-precision)" :default -5.0) (AltitudeHigh :type "Float (single-precision)" :default 5.0) (NAltitude :type Integer :default 3) (AzimuthLow :type "Float (single-precision)" :default 0.0) (AzimuthHigh :type "Float (single-precision)" :default 90.0) (NAzimuth :type Integer :default 20) (StructureRadius :type "Float (single-precision)" :default 10.0))
  (bind _bellhop (`self.Bellhop`))
  (bind _bellhop_2 (`self.Bellhop`))
  (`self.ClearRays`)
  (`BellhopController.SetRayMode` _bellhop_2)
  (`BellhopController.SetRayAltitudes` _bellhop_2 (`local.AltitudeLow`) (`local.AltitudeHigh`) (`local.NAltitude`))
  (`BellhopController.SetRayAzimuths` _bellhop_2 (`local.AzimuthLow`) (`local.AzimuthHigh`) (`local.NAzimuth`))
  (`BellhopController.RunBellhop` _bellhop)
  (for _index (range (`BellhopController.GetNRays` _bellhop))
    (bind _returnvalue (`|SpawnActorFromClass` "/Script/bellhop.FollowRays" (`self.GetTransform`) "Undefined" "MultiplyWithRoot" null null))
    (`FollowRays.CreateStructure` _returnvalue _index "/Game/Bottom/M_UnlitWhite.M_UnlitWhite" (`local.StructureRadius`))
    (set `FollowRays.WorldParameters` "/Game/Assets/MP_TransmissionLoss3D.MP_TransmissionLoss3D" _returnvalue)))

(fn `UserConstructionScript`)